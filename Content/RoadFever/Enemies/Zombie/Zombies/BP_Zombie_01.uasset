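; Zombie enemy that turns toward the player, moans, bleeds when hit and dies with a random animation.
; Tick finds a nav path to the player and eases yaw toward its next point while alive and unpaused; no translation happens here.
; Moans replay after random delays, continuing past death only when IsMeme is set.
; Damage calls the parent, prints debug text and spawns neck blood; Die disables capsule collision and adds delayed blood.
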(event `self.ReceiveTick`
  (params (DeltaSeconds :type "Float (single-precision)"))
  ;[1 1 1] AI Follow Player.
  (if (`self.isDead`)
    _
    (elif (not (`self.PlayerIsPaused`))
      (bind _returnvalue (`NavigationSystem.FindPathToLocationSynchronously` (`self.K2_GetActorLocation`) (`self.K2_GetActorLocation` (`GameplayStatics.GetPlayerPawn` 0)) null "/Script/Engine.RecastFilter_UseDefaultArea"))
      (bind (_returnvalue_roll _returnvalue_pitch _returnvalue_yaw) (`KismetMathLibrary.BreakRotator` (`KismetMathLibrary.FindLookAtRotation` (`self.K2_GetActorLocation`) (`KismetArrayLibrary.Array_Get` (`NavigationPath.PathPoints` _returnvalue) 1))))
      (`self.K2_SetActorRotation` (`KismetMathLibrary.RInterpTo` (`self.K2_GetActorRotation`) (`KismetMathLibrary.MakeRotator` 0.0 0.0 _returnvalue_yaw) (`GameplayStatics.GetWorldDeltaSeconds`) 1.0)))))

(event `self.ReceiveBeginPlay`
  ;[1 1 1] Moans.
  (`parent.ReceiveBeginPlay`)
  (`KismetSystemLibrary.Delay` (`KismetMathLibrary.RandomFloatInRange` 5.0 15.0))
  (if (`self.isDead`)
    (if (`self.isMeme`)
      (`ActorComponent.Activate` (`self.Moans`) false :!label _label))
    (else
      (goto _label))))

(event `self.Die`
  ;[1 1 1] Death Animation.
  (set `self.isDead` true)
  (`SkeletalMeshComponent.PlayAnimation` (`self.Mesh`) (`KismetArrayLibrary.Array_Get` (`|MakeArray` "/Game/RoadFever/Enemies/Zombie/Zombies/Death_1_Copy.Death_1_Copy" "/Game/RoadFever/Enemies/Zombie/Zombies/Death_2_Copy.Death_2_Copy" "/Game/RoadFever/Enemies/Zombie/Zombies/RootMotionAnimations/RootMotion/Zombie_Death_Back_Mid_1_Copy.Zombie_Death_Back_Mid_1_Copy" "/Game/RoadFever/Enemies/Zombie/Zombies/Idle_Knockdown_Front_Copy_Copy.Idle_Knockdown_Front_Copy_Copy" "/Game/RoadFever/Enemies/Zombie/Zombies/Idle_Knockdown_Left_Copy_Copy.Idle_Knockdown_Left_Copy_Copy" "/Game/RoadFever/Enemies/Zombie/Zombies/Idle_Knockdown_Right_Copy_Copy.Idle_Knockdown_Right_Copy_Copy" :!type "AnimationAsset Object Reference") (`KismetMathLibrary.RandomIntegerInRange` 0 5)) false)
  (`PrimitiveComponent.SetCollisionEnabled` (`self.CapsuleComponent`) "NoCollision")
  (`KismetSystemLibrary.Delay` 2.0)
  (`GameplayStatics.SpawnEmitterAttached` "/Game/RoadFever/Effects/Blood/P_Blood.P_Blood" (`self.Mesh`) "neck_01" (0.0 0.0 0.0) (struct) "SnapToTarget"))

(event `self.Moans.OnAudioFinished`
  ;[1 1 1] Moans.
  (`KismetSystemLibrary.Delay` (`KismetMathLibrary.RandomFloatInRange` 10.0 15.0))
  (if (`self.isDead`)
    (if (`self.isMeme`)
      (`AudioComponent.Play` (`self.Moans`) 0.0 :!label _label_2))
    (else
      (goto _label_2))))

(event `self.TakeDamage`
  (params (InDamage :type Integer))
  ;[1 1 1] Spawns an emitter but somewhat poorly.
  (`parent.TakeDamage` InDamage)
  (`KismetSystemLibrary.PrintString` "Get in the back of the van!")
  (`GameplayStatics.SpawnEmitterAttached` "/Game/RoadFever/Effects/Blood/P_Blood.P_Blood" (`self.Mesh`) "neck_01" (0.0 0.0 0.0) (struct) "SnapToTarget")
  (`KismetSystemLibrary.PrintString` "Zombie is bleeding." true true (struct :`R` 1.0 :`G` 0.434411 :`A` 1.0)))

(fn `UserConstructionScript`)